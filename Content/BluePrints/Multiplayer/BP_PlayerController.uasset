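; BP_PlayerController is the multiplayer player controller that passes player settings to the server and requests spawning and respawning.
; On BeginPlay it polls with a short delay until PlayerState is valid, then the local controller sends GameInstance settings to BP_PlayerState and requests a spawn from BP_GameMode.
; Once respawn is enabled, pressing P removes the stored widget and requests another spawn.
; Possession caches the pawn reference.
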(event Custom|SendPlayerSettings_Server
  (params (SetTo :type Struct%20Player%20Settings%20Structure))
  (bind _playerstate (Variables|GetPlayerState)
    (:then
      (bind _asbp_player_state (Utilities|Casting|CastToBP_PlayerState _playerstate))
      (Variables|/Game/BluePrints/Multiplayer/BP_PlayerState.BP_PlayerState_C|SetPlayerSettings _asbp_player_state SetTo))
    (:else)))

(event Custom|SpawnPlayer_Server
  (bind _asbp_game_mode (Utilities|Casting|CastToBP_GameMode (Game|GetGameMode)))
  (Default|ManagePlayerSpawn _asbp_game_mode self))

(event Custom|EnableRespawn
  (Variables|Default|Setrespawnable true))

(event Custom|EnableRespawnAndClearWidget
  (params (widgetToClear :type User%20Widget%20Object%20Reference))
  (Variables|Default|SetwidgetToClear widgetToClear)
  (CallFunction|EnableRespawn))

(event EventPossess
  (params (PossessedPawn :type Pawn%20Object%20Reference))
  (Variables|Default|SetPawnRef PossessedPawn))

(event EventBeginPlay
  (Variables|GetPlayerState :!label _label
    (:then
      (if (Pawn|IsLocalPlayerController)
        (bind _asbp_game_instance (Utilities|Casting|CastToBP_GameInstance (Game|GetGameInstance)))
        (CallFunction|SendPlayerSettingsServer (Variables|/Game/BluePrints/Multiplayer/BP_GameInstance.BP_GameInstance_C|GetPlayerSettings _asbp_game_instance))
        (Variables|Default|SetsettingsReady true)
        (CallFunction|SpawnPlayerServer)))
    (:else
      (Utilities|FlowControl|Delay 0.2)
      (goto _label))))

(event Input|KeyboardEvents|P
  (params (Key :type Key%20Structure :default "None"))
  (:Pressed
    (if (Variables|Default|Getrespawnable)
      (Variables|Default|Setrespawnable false)
      (Widget|RemovefromParent (Variables|Default|GetwidgetToClear))
      (CallFunction|SpawnPlayerServer))))

(fn ConstructionScript)