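; Tank character Blueprint that adds a charged high jump and wall climbing to its parent character.
; Holding Crouch on the ground builds charge in a Delay loop that updates a widget bar; pressing Jump launches high through a server event when nearly full, otherwise jumps normally.
; A looping timer traces forward from the feet and, while W is held, routes upward launches through server and multicast events.
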(event Custom|PerformJump_Server
  (if (Character|CanJump)
    (Character|LaunchCharacter "0, 0,1500.000000" false false)))

(event Custom|WallClimb_Multi
  (Variables|/Script/Engine.MovementComponent|SetVelocity (Variables|Character|GetCharacterMovement) "0, 0, 0")
  (Character|LaunchCharacter "0, 0,300.000000" false true))

(event Custom|WallClimb_Server
  (CallFunction|WallClimbMulti))

(event Custom|Wall%20Climb
  (bind _feet (Variables|Default|GetFeet))
  (bind _returnvalue (Transformation|GetWorldLocation _feet))
  (bind _returnvalue_2 (Collision|LineTraceByChannel _returnvalue (+ _returnvalue (* (Math|Vector|GetForwardVector (Transformation|GetWorldRotation _feet)) 2e+01)) "TraceTypeQuery1" false 0 "None"))
  (if _returnvalue_2
    (if (Game|Player|IsInputKeyDown (Game|GetPlayerController 0) "W")
      (CallFunction|WallClimbServer))))

(event EventBeginPlay
  (|CallParentFunction)
  (Utilities|Time|SetTimerbyEvent (delegate Custom|Wall%20Climb) 0.1 true))

(event Input|ActionEvents|InputActionCrouch
  (params (Key :type Key%20Structure :default "None"))
  (bind _jumpchargetime (Variables|Default|GetJumpChargeTime))
  (bind _widgetreference (Variables|Default|GetWidgetReference))
  (bind _jumpiterationtime (Variables|Default|GetJumpIterationTime))
  (bind _jumpchargetime_2 (Variables|Default|GetJumpChargeTime))
  (:Pressed
    (if (AI|Components|NavMovement|IsMovingonGround (Variables|Character|GetCharacterMovement))
      (bind _output_get (Variables|Default|SetCrouched true))
      (if _output_get :!label _label
        (Utilities|FlowControl|Delay _jumpiterationtime)
        (if _output_get
          (bind _output_get_2 (Variables|Default|SetJumpChargeProgress (+ (Variables|Default|GetJumpChargeProgress) _jumpiterationtime)))
          (if (>= (Math|Float|Min(Float) _output_get_2 _jumpchargetime_2) _jumpchargetime_2)
            (Class|ISetChargebarValue|SetChargebarValue(Message) _widgetreference _jumpchargetime _jumpchargetime)
            (else
              (Class|ISetChargebarValue|SetChargebarValue(Message) _widgetreference (Variables|Default|GetJumpChargeProgress) _jumpchargetime)
              (goto _label)))))))
  (:Released
    (Variables|Default|SetCrouched false)
    (bind _output_get_3 (Variables|Default|SetJumpChargeProgress 0.0))
    (Class|ISetChargebarValue|SetChargebarValue(Message) (Variables|Default|GetWidgetReference) _output_get_3 1.0)))

(event Input|ActionEvents|InputActionJump
  (params (Key :type Key%20Structure :default "None"))
  (:Pressed
    (Variables|Default|SetCrouched false)
    (Class|ISetChargebarValue|SetChargebarValue(Message) (Variables|Default|GetWidgetReference) 0.0 1.0)
    (if (>= (Variables|Default|GetJumpChargeProgress) (- (Variables|Default|GetJumpChargeTime) (Variables|Default|GetJumpChargeTolerance)))
      (Variables|Default|SetJumpChargeProgress 0.0)
      (CallFunction|PerformJumpServer)
      (else
        (Variables|Default|SetJumpChargeProgress 0.0)
        (Character|Jump)))))

(fn ConstructionScript
  (|CallParentFunction))

(fn TickJump
  (params (DeltaSeconds :type Float%20%28double-precision%29)))

(fn PerformJump
  (if (Character|CanJump)
    (Character|LaunchCharacter "0, 0,1500.000000" false false)))

(fn GetJumpCharge
  (return (Variables|Default|GetJumpChargeProgress)))