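; BP_MiscChar is a character with a cooldown-gated grapple and a wall climb, both routed through server and multicast events.
; Left Shift or right mouse sphere-traces from the camera, then a timeline lerps the actor to just short of the hit.
; A looping timer recharges the grapple, and its RepNotify updates the widget charge bar.
; Another timer line-traces from the feet, launching the character upward while W is held against a surface.
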(event Custom|Grappling_Multi
  (params (AttachPoint :type Vector))
  (Variables|Default|SetStart%20Point (Transformation|GetActorLocation))
  (bind _newtrack_1 (Timeline|Grapple PlayFromStart)
    (:Update
      (Transformation|SetActorLocation (Math|Vector|Lerp(Vector) (Variables|Default|GetStart%20Point) AttachPoint _newtrack_1) false false))))

(event Custom|GrappleSphereCheck_Server
  (bind _firstpersoncamera (Variables|Default|GetFirstPersonCamera))
  (bind _returnvalue (Transformation|GetWorldLocation _firstpersoncamera))
  (bind _returnvalue_2 (Math|Vector|GetForwardVector _firstpersoncamera))
  (if (>= (Variables|Default|GetGrappleValue) (Variables|Default|GetGrappleCooldown))
    (bind (_outhit _returnvalue_3) (Collision|SphereTraceByChannel _returnvalue (+ _returnvalue (* _returnvalue_2 (Variables|Default|GetGrappleRange))) 0.0 "TraceTypeQuery1" false 0 "ForDuration"))
    (if _returnvalue_3
      (Variables|Default|SetGrappleValue 0.0)
      (CallFunction|GrapplingMulti (+ (.Location (Collision|BreakHitResult _outhit)) (* _returnvalue_2 -55.0))))))

(event Custom|WallClimb_Multi
  (Variables|/Script/Engine.MovementComponent|SetVelocity (Variables|Character|GetCharacterMovement) "0, 0, 0")
  (Character|LaunchCharacter "0, 0,300.000000" false true))

(event Custom|WallClim_Server
  (CallFunction|WallClimbMulti))

(event Custom|addToTimer
  (CallFunction|AddtoTimerServer))

(event Custom|Wall%20Climb
  (bind _feet (Variables|Default|GetFeet))
  (bind _returnvalue (Transformation|GetWorldLocation _feet))
  (bind _returnvalue_2 (Collision|LineTraceByChannel _returnvalue (+ _returnvalue (* (Math|Vector|GetForwardVector (Transformation|GetWorldRotation _feet)) 2e+01)) "TraceTypeQuery1" false 0 "None"))
  (if _returnvalue_2
    (if (Game|Player|IsInputKeyDown (Game|GetPlayerController 0) "W")
      (CallFunction|WallClimServer))))

(event Custom|addToTimer_Server
  (Variables|Default|SetGrappleValue (Math|Float|Min(Float) (+ (Variables|Default|GetGrappleValue) 0.1) (Variables|Default|GetGrappleCooldown))))

(event EventBeginPlay
  (|CallParentFunction)
  (Utilities|Time|SetTimerbyEvent (delegate Custom|Wall%20Climb) 0.1 true)
  (Utilities|Time|SetTimerbyEvent (delegate Custom|addToTimer) 0.1 true))

(event Input|MouseEvents|RightMouseButton
  (params (Key :type Key%20Structure :default "None"))
  (:Pressed
    (CallFunction|GrappleSphereCheckServer)))

(event Input|KeyboardEvents|LeftShift
  (params (Key :type Key%20Structure :default "None"))
  (:Pressed
    (CallFunction|GrappleSphereCheckServer)))

(fn ConstructionScript
  (|CallParentFunction))

(fn OnRepGrappleValue
  (Class|ISetChargebarValue|SetChargebarValue(Message) (Variables|Default|GetWidgetReference) (Variables|Default|GetGrappleValue) (Variables|Default|GetGrappleCooldown)))