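; Agile first-person character, extending a parent character, with a cooldown-limited dash and wall climbing.
; Dash line-traces along movement input or camera forward, stops short of hits, lerps the actor there on a timeline, then sets exit velocity.
; Looping timers refill the dash charge bar and poll a feet trace, launching the character upward while W is held against a surface.
; Both moves are relayed through Server-to-Multi events.
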(event Custom|Dash_Server
  (params (Dash%20Direction :type Vector) (Dash%20Velocity :type Vector))
  (CallFunction|DashMulti Dash%20Direction Dash%20Velocity))

(event Custom|Dash_Multi
  (params (DashDirection :type Vector) (DashVelocity :type Vector))
  (CallFunction|ResetDashTimer)
  (bind _alpha (Timeline|Timeline_0 PlayFromStart)
    (:Update
      (Transformation|SetActorLocation (Math|Vector|Lerp(Vector) (Transformation|GetActorLocation) DashDirection _alpha) false false))
    (:Finished
      (Variables|/Script/Engine.MovementComponent|SetVelocity (Variables|Character|GetCharacterMovement) (* DashVelocity 5e+02)))))

(event Custom|WallClimb_Server
  (CallFunction|WallClimbMulti))

(event Custom|Wall%20Climb
  (bind _feet (Variables|Default|GetFeet))
  (bind _returnvalue (Transformation|GetWorldLocation _feet))
  (bind _returnvalue_2 (Collision|LineTraceByChannel _returnvalue (+ _returnvalue (* (Math|Vector|GetForwardVector (Transformation|GetWorldRotation _feet)) 2e+01)) "TraceTypeQuery1" false 0 "None"))
  (if _returnvalue_2
    (if (Game|Player|IsInputKeyDown (Game|GetPlayerController 0) "W")
      (CallFunction|WallClimbServer))))

(event Custom|WallClimb_Multi
  (Variables|/Script/Engine.MovementComponent|SetVelocity (Variables|Character|GetCharacterMovement) "0, 0, 0")
  (Character|LaunchCharacter "0, 0,300.000000" false true))

(event Custom|DashTimer
  (bind _dashcooldown (Variables|Default|GetDashCooldown))
  (if (not (Variables|Default|GetCanDash))
    (bind _output_get (Variables|Default|SetDashTimerProgress (+ (Variables|Default|GetDashTimerProgress) (Variables|Default|GetDashTimerIterationTime))))
    (bind _output_get_2 (Variables|Default|SetDashTimerProgress (Math|Float|SelectFloat _dashcooldown _output_get (>= _output_get _dashcooldown))))
    (Variables|Default|SetCanDash (>= _output_get _dashcooldown))
    (Class|ISetChargebarValue|SetChargebarValue(Message) (Variables|Default|GetWidgetReference) _output_get_2 (Variables|Default|GetDashCooldown))))

(event EventBeginPlay
  (|CallParentFunction)
  (Utilities|Time|SetTimerbyEvent (delegate Custom|Wall%20Climb) 0.1 true)
  (Utilities|Time|SetTimerbyEvent (delegate Custom|DashTimer) (Variables|Default|GetDashTimerIterationTime) true))

(event Input|ActionEvents|InputActionDash
  (params (Key :type Key%20Structure :default "None"))
  (bind _returnvalue (Transformation|GetActorLocation))
  (bind _returnvalue_2 (Transformation|GetActorLocation))
  (bind _firstpersoncamera (Variables|Default|GetFirstPersonCamera))
  (bind _charactermovement (Variables|Character|GetCharacterMovement))
  (bind _charactermovement_2 (Variables|Character|GetCharacterMovement))
  (bind _returnvalue_3 (Pawn|Components|PawnMovement|GetLastInputVector _charactermovement))
  (bind _returnvalue_4 (Pawn|Components|PawnMovement|GetLastInputVector _charactermovement_2))
  (bind _returnvalue_5 (Math|Vector|GetForwardVector _firstpersoncamera))
  (bind _returnvalue_6 (Math|Vector|MakeVector (.x _returnvalue_5) (.y _returnvalue_5) (.z _returnvalue_5)))
  (bind _returnvalue_7 (Math|Vector|Normalize _returnvalue_6))
  (:Pressed
    (if (Variables|Default|GetCanDash)
      (if (and (not (Utilities|Operators|EqualEqual (Transformation|GetActorForwardVector) _returnvalue_3 1.0)) (Class|AIBlueprintHelperLibrary|IsValidAIDirection _returnvalue_3))
        (bind (_outhit _returnvalue_8) (Collision|LineTraceByChannel _returnvalue (+ _returnvalue (* _returnvalue_3 5e+02)) "TraceTypeQuery1" false 0 "None"))
        (if _returnvalue_8
          (CallFunction|DashServer (+ (.Location (Collision|BreakHitResult _outhit)) (* _returnvalue_3 -55.0)) _returnvalue_4)
          (else
            (CallFunction|DashServer (.TraceEnd (Collision|BreakHitResult _outhit)) _returnvalue_4)))
        (else
          (bind (_outhit_2 _returnvalue_9) (Collision|LineTraceByChannel _returnvalue_2 (+ _returnvalue_2 (* _returnvalue_7 5e+02)) "TraceTypeQuery1" false 0 "None"))
          (if _returnvalue_9
            (CallFunction|DashServer (+ (.Location (Collision|BreakHitResult _outhit_2)) (* _returnvalue_7 -55.0)) _returnvalue_7)
            (else
              (CallFunction|DashServer (.TraceEnd (Collision|BreakHitResult _outhit_2)) "0, 0, 0"))))))))

(fn ConstructionScript
  (|CallParentFunction))

(fn ResetDashTimer
  (Variables|Default|SetDashTimerProgress 0.0)
  (Variables|Default|SetCanDash false)
  (Class|ISetChargebarValue|SetChargebarValue(Message) (Variables|Default|GetWidgetReference) 0.0 1.0))